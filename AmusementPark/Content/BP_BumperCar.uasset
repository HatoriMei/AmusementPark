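; BP_BumperCar is a player-driven bumper car controlled through Enhanced Input actions.
; IA_CarMove pushes the static mesh along its forward vector with a physics force scaled by MoveForce and the input value.
; IA_CarTurn steers by setting the mesh's world yaw directly from TurnSpeed and input, zeroing pitch and roll instead of applying torque.
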(event `EnhancedInput|/Game/IA_CarMove`
  (params (ActionValue :type "Float (double-precision)") (ElapsedSeconds :type "Float (double-precision)") (TriggeredSeconds :type "Float (double-precision)") (InputAction :type "InputAction Object Reference" :default "/Game/IA_CarMove.IA_CarMove"))
  (bind _staticmesh (`self.StaticMesh`))
  (:`Triggered`
    (`PrimitiveComponent.AddForce` _staticmesh (* (`SceneComponent.GetForwardVector` _staticmesh) (`self.MoveForce`) ActionValue) "None" false)))

(event `EnhancedInput|/Game/IA_CarTurn`
  (params (ActionValue :type "Float (double-precision)") (ElapsedSeconds :type "Float (double-precision)") (TriggeredSeconds :type "Float (double-precision)") (InputAction :type "InputAction Object Reference" :default "/Game/IA_CarTurn.IA_CarTurn"))
  (bind _staticmesh (`self.StaticMesh`))
  (bind (_returnvalue_roll _returnvalue_pitch _returnvalue_yaw) (`KismetMathLibrary.BreakRotator` (`SceneComponent.K2_GetComponentRotation` _staticmesh)))
  (:`Triggered`
    (`SceneComponent.K2_SetWorldRotation` _staticmesh (`KismetMathLibrary.MakeRotator` 0.0 0.0 (+ _returnvalue_yaw (* ActionValue (`self.TurnSpeed`)))) false false)))

(fn `UserConstructionScript`)