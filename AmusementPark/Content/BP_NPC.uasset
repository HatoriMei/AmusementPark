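; BP_NPC is an NPC that wanders between randomly chosen BP_Target actors until it is destroyed.
; On BeginPlay it caches every BP_Target, then Move picks one at random and switches on its Type.
; Regular targets trigger AIMoveTo and another pick on success or failure, while Creation targets cause an immediate re-pick.
; Picking a Destruction target destroys the NPC at once, without moving to it.
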(event `self.ReceiveBeginPlay`
  (bind _outactors (`GameplayStatics.GetAllActorsOfClass` "/Game/BP_Target.BP_Target_C"))
  (set `self.TargetPoint` _outactors)
  (`self.Move` :!label _label))

(event `Move`
  (bind _output_get (set `self.Random TP` (`KismetArrayLibrary.Array_Random` (`self.TargetPoint`))))
  (switch `/Game/E_NavTargetPointType` (`/Game/BP_Target.Type` _output_get)
    (:`NewEnumerator0`
      (`self.K2_DestroyActor`))
    (:`NewEnumerator1`
      (goto _label))
    (:`NewEnumerator2`
      (`|AIMoveTo` self (`self.K2_GetActorLocation` (`self.Random TP`)) null
        (:`OnSuccess`
          (goto _label))
        (:`OnFail`
          (goto _label))))))

(fn `UserConstructionScript`)