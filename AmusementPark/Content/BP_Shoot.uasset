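; BP_Shoot gives its owning actor the ability to fire a physics-driven BP_Ball projectile.
; Its Shoot function spawns the ball a short fixed distance in front of the owner, along its forward vector.
; It then applies an impulse to the ball's Sphere in that same direction, scaled by the Impulse variable and affected by mass.
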(fn `Shoot`
  (bind _returnvalue (`self.GetOwner`))
  (bind _returnvalue_2 (`|SpawnActorFromClass` "/Game/BP_Ball.BP_Ball_C" (`KismetMathLibrary.MakeTransform` (+ (`Actor.K2_GetActorLocation` _returnvalue) (* (`Actor.GetActorForwardVector` _returnvalue) 80.0))) "Undefined" "MultiplyWithRoot" null null))
  (`PrimitiveComponent.AddImpulse` (`/Game/BP_Ball.Sphere` _returnvalue_2) (* (`Actor.GetActorForwardVector` (`self.GetOwner`)) (`self.Impulse`)) "None" false))