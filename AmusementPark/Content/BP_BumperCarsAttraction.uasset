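; Bumper cars attraction whose Box trigger switches the first player controller between the third-person character and a bumper car.
; When a Player-tagged actor enters, the controller possesses a random BP_BumperCar and adds the bumper car input mapping context.
; When any actor exits, it nudges that actor along negative Y, possesses a random BP_ThirdPersonCharacter, adds the default context and prints a debug string.
; Neither path removes the previous mapping context.
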(event `self.Box.OnComponentBeginOverlap`
  (params (OverlappedComponent :type "PrimitiveComponent Object Reference") (OtherActor :type "Actor Object Reference") (OtherComp :type "PrimitiveComponent Object Reference") (OtherBodyIndex :type Integer) (bFromSweep :type Boolean) (SweepResult :type "HitResult Structure (by ref)"))
  (bind _returnvalue (`GameplayStatics.GetPlayerController` 0))
  (if (`self.ActorHasTag` OtherActor "Player")
    (bind _outactors (`GameplayStatics.GetAllActorsOfClass` "/Game/BP_BumperCar.BP_BumperCar_C"))
    (bind _output_get (set `self.BumperCars` _outactors))
    (`Controller.Possess` _returnvalue (`KismetArrayLibrary.Array_Random` _output_get))
    (`EnhancedInputSubsystemInterface.AddMappingContext` (pcsubsystem `EnhancedInputLocalPlayerSubsystem` _returnvalue) "/Game/IMC_BumperCars.IMC_BumperCars" 0 (struct))))

(event `self.Box.OnComponentEndOverlap`
  (params (OverlappedComponent :type "PrimitiveComponent Object Reference") (OtherActor :type "Actor Object Reference") (OtherComp :type "PrimitiveComponent Object Reference") (OtherBodyIndex :type Integer))
  (bind _returnvalue (`GameplayStatics.GetPlayerController` 0))
  (bind (_returnvalue_x _returnvalue_y _returnvalue_z) (`KismetMathLibrary.BreakVector` (`self.K2_GetActorLocation` OtherActor)))
  (`self.K2_SetActorLocation` OtherActor (`KismetMathLibrary.MakeVector` _returnvalue_x (- _returnvalue_y 50.0) _returnvalue_z) false false)
  (bind _outactors (`GameplayStatics.GetAllActorsOfClass` "/Game/ThirdPerson/Blueprints/BP_ThirdPersonCharacter.BP_ThirdPersonCharacter_C"))
  (`Controller.Possess` _returnvalue (`KismetArrayLibrary.Array_Random` _outactors))
  (`EnhancedInputSubsystemInterface.AddMappingContext` (pcsubsystem `EnhancedInputLocalPlayerSubsystem` _returnvalue) "/Game/ThirdPerson/Input/IMC_Default.IMC_Default" 0 (struct))
  (`KismetSystemLibrary.PrintString` "Bloubibloup" true true (struct :`R` 0.097873 :`G` 0.854167 :`B` 0.418135 :`A` 1.0)))

(fn `UserConstructionScript`)